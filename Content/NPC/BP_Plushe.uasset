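; BP_Plushe is an AI-driven NPC that feeds its spawn location, master and perceived enemy to the blackboard through BP_AIController.
; On BeginPlay it caches the controller, stores its start location as the default and sets the first BP_Player found as master.
; Perception updates print the actor's name, then set any sensed actor as enemy without filtering, or clear the enemy when sensing fails.
; MakeFriendly is an empty stub.
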(event `self.ReceiveBeginPlay`
  (set `self.DefaultLocation` (`self.K2_GetActorLocation`))
  (bind _asbp_aicontroller (cast `/Game/NPC/BP_AIController` (`self.GetController`)))
  (bind _output_get (set `self.AIControllerRef` _asbp_aicontroller))
  (`/Game/NPC/BP_AIController.BB_SetDefaultLocation` _output_get (`self.DefaultLocation`))
  (bind _outactors (`GameplayStatics.GetAllActorsOfClass` "/Game/Player/BP_Player.BP_Player_C"))
  (`/Game/NPC/BP_AIController.BB_SetMaster` _output_get (`|GetArrayItem` _outactors)))

(event `self.AIPerception.OnTargetPerceptionUpdated`
  (params (Actor :type "Actor Object Reference") (Stimulus :type "AIStimulus Structure"))
  (`KismetSystemLibrary.PrintString` (`KismetSystemLibrary.GetDisplayName` Actor))
  (if (`.bSuccessfullySensed` (break `AIStimulus` Stimulus))
    (`self.OnEnemyDetected` Actor)
    (else
      (`self.OnEnemyLost` Actor))))

(event `OnEnemyDetected`
  (params (Actor :type "Actor Object Reference"))
  (`/Game/NPC/BP_AIController.BB_SetEnemy` (`self.AIControllerRef`) Actor))

(event `OnEnemyLost`
  (params (Actor :type "Actor Object Reference"))
  (`/Game/NPC/BP_AIController.BB_SetEnemy` (`self.AIControllerRef`) null))

(fn `MakeFriendly`)

(fn `UserConstructionScript`)